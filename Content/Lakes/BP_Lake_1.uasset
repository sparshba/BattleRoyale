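; BP_Lake_1 is a lake actor that deals environmental damage to players whose view point is under its water level.
; Each tick on the server, it loops over the battle royale game mode's alive player list.
; Any player with eye height at or below the actor's Z takes WaterDamageRate damage per second on their controlled pawn.
; The test compares height only, with no horizontal bounds or overlap volume.
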(event EventTick
  (params (DeltaSeconds :type Float%20%28single-precision%29))
  (Networking|SwitchHasAuthority
    (:Authority
      (bind _asbrgame_mode (Utilities|Casting|CastToBRGameMode (Game|GetGameMode)))
      (for _array_element (Variables|/Game/FirstPersonBP/Blueprints/BRGameMode.BRGameMode_C|GetAlive%20PlayerList _asbrgame_mode)
        (if (<= (.Z (Math|Vector|BreakVector (.OutLocation (Actor|GetActorEyesViewPoint _array_element)))) (.Z (Math|Vector|BreakVector (Transformation|GetActorLocation))))
          (Game|Damage|ApplyDamage (Pawn|GetControlledPawn _array_element) (* DeltaSeconds (Variables|Default|GetWaterDamageRate)) 0 self "/Engine/EngineDamageTypes/DmgTypeBP_Environmental.DmgTypeBP_Environmental_C"))))))

(fn ConstructionScript)