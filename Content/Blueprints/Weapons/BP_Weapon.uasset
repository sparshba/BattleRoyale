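; BP_Weapon is a weapon actor that tracks clip and spare ammo for its owning BPCharacter.
; On the authority it caches that owner at BeginPlay, spends a round per shot and calls Reload when the clip empties.
; Reload sets the owner's Reloading flag around a fixed delay, then refills the clip from spare ammo.
; GiveAmmo, also authority-only, tops up the clip before adding to capped reserves.
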(event Custom|Give%20Ammo
  (params (Ammo%20To%20Give :type Integer))
  ;[1 1 1] Event To Give Ammo To The Weapon When Needed
  (Networking|SwitchHasAuthority
    (:Authority
      (Variables|Ammo|SetCurrentAmmo (+ (Variables|Ammo|GetCurrentAmmo) (Math|Integer|Min(Integer) Ammo%20To%20Give (- (Variables|Ammo|GetClipSize) (Variables|Ammo|GetCurrentAmmo)))))
      (if (> (- Ammo%20To%20Give (Math|Integer|Min(Integer) Ammo%20To%20Give (- (Variables|Ammo|GetClipSize) (Variables|Ammo|GetCurrentAmmo)))) 0)
        (Variables|Ammo|SetCurrentSpareAmmo (+ (Variables|Ammo|GetCurrentSpareAmmo) (Math|Integer|Min(Integer) (- Ammo%20To%20Give (Math|Integer|Min(Integer) Ammo%20To%20Give (- (Variables|Ammo|GetClipSize) (Variables|Ammo|GetCurrentAmmo)))) (- (Variables|Ammo|GetMaxSpareAmmo) (Variables|Ammo|GetCurrentSpareAmmo)))))))))

(event Custom|On%20Fired
  (bind _currentammo (Variables|Ammo|GetCurrentAmmo))
  ;[1 1 1] When We Fire Our Gun Take Ammo From Player And Reload If Necessary
  (Networking|SwitchHasAuthority
    (:Authority
      (Math|Integer|DecrementInt _currentammo
        (:%20%20
          (if (<= _currentammo 0)
            (CallFunction|Reload)))))))

(event Custom|Reload
  ;[1 1 1] Reload The Weapon And Play Animation
  (Variables|/Game/FirstPersonBP/Blueprints/BPCharacter.BPCharacter_C|SetReloading? (Variables|Default|Get%20CurrentOwner) true)
  (Utilities|FlowControl|Delay 2.0)
  (Variables|Ammo|SetCurrentAmmo (Math|Integer|Min(Integer) (Variables|Ammo|GetCurrentSpareAmmo) (Variables|Ammo|GetClipSize)))
  (Variables|Ammo|SetCurrentSpareAmmo (Math|Integer|Max(Integer) (- (Variables|Ammo|GetCurrentSpareAmmo) (Math|Integer|Min(Integer) (Variables|Ammo|GetCurrentSpareAmmo) (Variables|Ammo|GetClipSize)))))
  (Variables|/Game/FirstPersonBP/Blueprints/BPCharacter.BPCharacter_C|SetReloading? (Variables|Default|Get%20CurrentOwner) false))

(event EventBeginPlay
  ;[1 1 1] On Begin Play Set Up Ammo Amount
  (Networking|SwitchHasAuthority
    (:Authority
      (bind _asbpcharacter (Utilities|Casting|CastToBPCharacter (Components|GetOwner)))
      (Variables|Default|Set%20CurrentOwner _asbpcharacter))))

(fn ConstructionScript)

(fn HasAmmo
  (return (> (Variables|Ammo|GetCurrentAmmo) 0)))