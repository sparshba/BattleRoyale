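; BP_HealthPickUp is a pickup that restores health to a character who enters its sphere.
; It handles the sphere-entered event on the authority only and ignores characters already at maximum health.
; Otherwise it passes a negated HealthToGive to the character's ModifyHealth, then destroys itself.
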(event EventPickUpSphereEntered
  (params (Character :type BP%20Character%20Object%20Reference))
  (Networking|SwitchHasAuthority
    (:Authority
      (if (< (Variables|/Game/FirstPersonBP/Blueprints/BPCharacter.BPCharacter_C|GetHealth Character) (Variables|/Game/FirstPersonBP/Blueprints/BPCharacter.BPCharacter_C|GetMaxHealth Character))
        (Default|ModifyHealth Character (* (Variables|Default|GetHealthToGive) -1.0))
        (Actor|DestroyActor)))))

(fn ConstructionScript
  (|CallParentFunction))