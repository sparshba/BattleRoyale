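; Weapon pickup actor that carries a weapon class along with its clip and spare ammo counts.
; On BeginPlay the authority fills ammo from the weapon's class defaults, unless a player dropped it, so dropped weapons keep their remaining ammo.
; Pickup sphere events register it as the character's current weapon pickup on entry and clear that reference on exit only if it still points to this pickup.
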(event EventPickUpSphereEntered
  (params (Character :type BP%20Character%20Object%20Reference))
  ;[1 1 1] SetPlayer PickUp
  (Variables|/Game/FirstPersonBP/Blueprints/BPCharacter.BPCharacter_C|SetCurrentWeaponPickup Character self))

(event EventPickUpSphereLift
  (params (Character :type BP%20Character%20Object%20Reference))
  ;[1 1 1] Unset PlayerPickUp
  (if (== (Variables|/Game/FirstPersonBP/Blueprints/BPCharacter.BPCharacter_C|GetCurrentWeaponPickup Character) self)
    (Variables|/Game/FirstPersonBP/Blueprints/BPCharacter.BPCharacter_C|SetCurrentWeaponPickup Character 0)))

(event EventBeginPlay
  (bind _weapontogive (Variables|Default|GetWeaponToGive))
  (bind (_damage _weaponname _currentammo _currentspareammo) (Utilities|GetClassDefaults _weapontogive))
  ;[1 1 1] Remember ammo amount if player dropped weapon
  (Networking|SwitchHasAuthority
    (:Authority
      (if (not (Variables|Default|GetDroppedByPlayer?))
        (Variables|Default|SetCurrentAmmoInClip _currentammo)
        (Variables|Default|SetCurrentSpareAmmo _currentspareammo)))))

(fn ConstructionScript
  (|CallParentFunction))