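; Battle royale safe zone that registers on BRGameState and shrinks in stages, damaging players outside its wall.
; Once enabled, server timers alternate holds with shrinks, picking a random next center and scaling radius and timings until below MinRadius.
; Tick scales and moves the actor, with Radius serving as wall diameter.
; The server applies environmental damage by horizontal distance to alive players off the plane while the wall is visible.
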(event Custom|Enable%20Safe%20Zone
  (Networking|SwitchHasAuthority
    (:Authority
      (Variables|Default|SetEnabled? true)
      (Utilities|Time|SetTimerbyEvent (delegate Custom|Begin%20Shrinking) (Variables|Default|GetHold%20Time)))))

(event Custom|Begin%20Shrinking
  (Networking|SwitchHasAuthority
    (:Authority
      (Math|Integer|IncrementInt (Variables|Default|GetNumShrinks)
        (:%20%20
          (Variables|Default|SetStartShrinkLocation (Transformation|GetActorLocation))
          (Variables|Default|SetShrinking? true)
          (Variables|Default|SetBeginShrinkingTime (Utilities|Time|GetTimeSeconds))
          (Variables|Default|SetShrinkSpeed (/ (- (Variables|Default|GetRadius) (Variables|Default|GetNextRadius)) (Variables|Default|GetShrinkTime)))
          (Rendering|SetActorHiddenInGame false))))))

(event Custom|Damage%20Players%20Outside%20Wall
  (params (Delta%20Seconds :type Float%20%28single-precision%29))
  (if (Math|Boolean|ANDBoolean (Variables|Default|GetEnabled?) (>= (Variables|Default|GetNumShrinks) 0) (not (Variables|Rendering|GetbHidden)))
    (bind _asbrgame_mode (Utilities|Casting|CastToBRGameMode (Game|GetGameMode)))
    (for _array_element (Variables|/Game/FirstPersonBP/Blueprints/BRGameMode.BRGameMode_C|GetAlive%20PlayerList _asbrgame_mode)
      (if (and (not (Variables|/Game/FirstPersonBP/Blueprints/BRPlayerController.BRPlayerController_C|GetIsOnPlane? _array_element)) (> (Transformation|GetHorizontalDistanceTo (Pawn|GetControlledPawn _array_element)) (/ (Variables|Default|GetRadius) 2.0)))
        (Game|Damage|ApplyDamage (Pawn|GetControlledPawn _array_element) (* (Variables|Default|GetWallDamagePerSecond) Delta%20Seconds) 0 self "/Engine/EngineDamageTypes/DmgTypeBP_Environmental.DmgTypeBP_Environmental_C")))))

(event Custom|UpdateWall%20Transform
  (params (Delta%20Seconds :type Float%20%28single-precision%29))
  ;[1 1 1] Comment
  (Variables|Default|SetRadius (- (Variables|Default|GetRadius) (* (Variables|Default|GetShrinkSpeed) Delta%20Seconds)))
  (Transformation|SetActorScale3D (Math|Vector|MakeVector (Variables|Default|GetRadius) (Variables|Default|GetRadius) (Variables|Default|GetHeight)))
  (Transformation|SetActorLocation (Math|Interpolation|VInterptoConstant (Transformation|GetActorLocation) (Variables|Default|GetNextLocation) Delta%20Seconds (/ (Math|Vector|VectorLength (- (Variables|Default|GetStartShrinkLocation) (Variables|Default|GetNextLocation))) (Variables|Default|GetShrinkTime))) false false)
  (if (and (Ability|HasAuthority) (>= (/ (- (Utilities|Time|GetTimeSeconds) (Variables|Default|GetBeginShrinkingTime)) (Variables|Default|GetShrinkTime)) 1.0))
    (Variables|Default|SetShrinking? false)
    (Variables|Default|SetHold%20Time (* (Variables|Default|GetHold%20Time) (Variables|Default|GetTimeMultiplier)))
    (Variables|Default|SetNextRadius (* (Variables|Default|GetNextRadius) (Variables|Default|GetShrinkMultiplier)))
    (Variables|Default|SetNextLocation (CallFunction|GetNextLocation))
    (Variables|Default|SetShrinkTime (* (Variables|Default|GetShrinkTime) (Variables|Default|GetShrinkMultiplier)))
    (if (>= (Variables|Default|GetRadius) (Variables|Default|GetMinRadius))
      (Utilities|Time|SetTimerbyEvent (delegate Custom|Begin%20Shrinking) (Variables|Default|GetHold%20Time))
      (else
        (Variables|Default|SetFinishShrinking? true)))))

(event EventBeginPlay
  (Networking|SwitchHasAuthority
    (:Authority
      (bind _asbrgame_state (Utilities|Casting|CastToBRGameState (Game|GetGameState)))
      (Variables|/Game/FirstPersonBP/Blueprints/BRGameState.BRGameState_C|SetSafeZone _asbrgame_state self)
      (Variables|Default|SetNextRadius (* (Variables|Default|GetRadius) (Variables|Default|GetShrinkMultiplier)))
      (Variables|Default|SetShrinkSpeed (/ (- (Variables|Default|GetRadius) (Variables|Default|GetNextRadius)) (Variables|Default|GetShrinkTime)))
      (Variables|Default|SetNextLocation (CallFunction|GetNextLocation)))))

(event EventTick
  (params (DeltaSeconds :type Float%20%28single-precision%29))
  (if (Variables|Default|GetShrinking?)
    (CallFunction|UpdateWallTransform DeltaSeconds))
  (if (Variables|Default|GetEnabled?)
    (Networking|SwitchHasAuthority
      (:Authority
        (CallFunction|DamagePlayersOutsideWall DeltaSeconds)))))

(fn ConstructionScript
  (bind _radius (Variables|Default|GetRadius))
  (Transformation|SetWorldScale3D (Variables|Default|GetWallMesh) (Math|Vector|MakeVector _radius _radius (Variables|Default|GetHeight))))

(fn GetNextLocation
  (bind _returnvalue (Math|Random|RandomFloatinRange -1.8e+02 1.8e+02))
  (bind _returnvalue_2 (Math|Random|RandomFloatinRange -1.8e+02 1.8e+02))
  (bind _returnvalue_3 (Transformation|GetActorLocation))
  (bind _radius (Variables|Default|GetRadius))
  (bind _nextradius (Variables|Default|GetNextRadius))
  (bind _returnvalue_4 (- _radius _nextradius))
  (bind _returnvalue_5 (Math|Trig|Cos(Degrees) _returnvalue_2))
  (bind _returnvalue_6 (Math|Trig|Sin(Degrees) _returnvalue))
  (bind _z (Math|Vector|BreakVector _returnvalue_3))
  (bind _returnvalue_7 (* _returnvalue_4 0.5))
  (bind _returnvalue_8 (* _returnvalue_7 -1.0))
  (bind _returnvalue_9 (Math|Random|RandomFloatinRange _returnvalue_8 _returnvalue_7))
  (bind _returnvalue_10 (Math|Random|RandomFloatinRange _returnvalue_8 _returnvalue_7))
  (bind _returnvalue_11 (* _returnvalue_6 _returnvalue_9))
  (bind _returnvalue_12 (* _returnvalue_5 _returnvalue_10))
  (bind _returnvalue_13 (Math|Vector|MakeVector _returnvalue_12 _returnvalue_11 _z))
  (bind _returnvalue_14 (+ _returnvalue_3 _returnvalue_13))
  (bind (_x _y) (Math|Vector|BreakVector _returnvalue_14))
  (return (Math|Vector|MakeVector _x _y _z)))